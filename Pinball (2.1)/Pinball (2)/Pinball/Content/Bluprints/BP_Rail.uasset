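; BP_Rail is a spline-based rail actor that appears unfinished, with no active runtime logic.
; Its construction script loops over the spline's segments but adds a spline mesh component only for the first one, without setting its start and end.
; A disconnected branch holds the logic to add a mesh and fit it to each segment's local point locations and tangents, but it never runs.
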(fn `UserConstructionScript`
  (for _index (range (+ (- (`SplineComponent.GetNumberOfSplinePoints` (`self.Spline`)) 2) 1))
    (if (== _index 0)
      (`AddComponent|NODE_AddSplineMeshComponent-1`))))