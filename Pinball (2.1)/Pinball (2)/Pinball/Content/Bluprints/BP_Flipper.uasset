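; BP_Flipper is a flipper actor, configurable as left or right, that swings between a rest and a flipped rotation.
; The construction script picks mirrored start and end rotations from the Flip setting and poses the Flipper component at rest.
; FlipEvent snaps it to the end rotation with MoveComponentTo, and FlopEvent returns it more slowly.
; An unconnected flip/flop delay loop never runs, so both events need external callers.
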(event `self.ReceiveBeginPlay`)

(event `FlipEvent`
  (`KismetSystemLibrary.MoveComponentTo` (`self.Flipper`) (0.0 0.0 0.0) (`self.EndRot`) false false 0.02))

(event `FlopEvent`
  (`KismetSystemLibrary.MoveComponentTo` (`self.Flipper`) (0.0 0.0 0.0) (`self.StartRot`) false false 0.1))

(fn `UserConstructionScript`
  (set `self.StartRot` (select `/Game/Bluprints/FlipType` (`self.Flip`) :`NewEnumerator0` (struct :`Yaw` -70.0) :`NewEnumerator1` (struct :`Yaw` 70.0) :!type "Rotator Structure"))
  (set `self.EndRot` (select `/Game/Bluprints/FlipType` (`self.Flip`) :`NewEnumerator0` (struct :`Yaw` -110.0) :`NewEnumerator1` (struct :`Yaw` 110.0) :!type "Rotator Structure"))
  (`SceneComponent.K2_SetRelativeRotation` (`self.Flipper`) (`self.StartRot`) false false))