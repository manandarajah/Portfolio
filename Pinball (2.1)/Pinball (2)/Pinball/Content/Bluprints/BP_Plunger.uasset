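; Plunger actor that pulls back while charging and snaps forward on release, with a reference position for the ball.
; ChargePlunger plays the PlayCharge timeline from the start, lerping the Plunger component back along its local X axis.
; StopCharge halts the timeline and uses MoveComponentTo to quickly return the component to its relative origin.
; GetBallLocation returns the actor location plus the BallLocation offset, without applying actor rotation.
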(event `ChargePlunger`
  (bind (_direction _charge) (`Timeline|PlayCharge` :!via `PlayFromStart` :!label _label)
    (:`Update`
      (`SceneComponent.K2_SetRelativeLocation` (`self.Plunger`) (`KismetMathLibrary.VLerp` (0.0 0.0 0.0) (-1500.0 0.0 0.0) _charge) false false))))

(event `StopCharge`
  (`|ExecutionSequence`
    (:`then_0`
      (goto _label :!via `Stop`))
    (:`then_1`
      (`KismetSystemLibrary.MoveComponentTo` (`self.Plunger`) (0.0 0.0 0.0) (`SceneComponent.RelativeRotation` (`self.Plunger`)) false false 0.1))))

(fn `GetBallLocation`
  (returns (BallAbsoluteLocation :type "Vector Structure"))
  (return (+ (`self.K2_GetActorLocation`) (`self.BallLocation`))))

(fn `UserConstructionScript`)