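; BP_Ball is a physics-driven ball actor that pushes itself along world negative X and pulls itself toward surfaces beneath it.
; Each Tick adds a DownwardForce velocity-change impulse on negative X, independent of mass and not scaled by delta time.
; A 2000-unit downward Visibility trace, left with persistent debug drawing, adds a StickyNess impulse on negative Z whenever it hits.
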(event `self.ReceiveTick`
  (params (DeltaSeconds :type "Float (single-precision)"))
  (bind _returnvalue (`self.K2_GetActorLocation`))
  (`PrimitiveComponent.AddImpulse` (`self.Ball`) (`KismetMathLibrary.MakeVector` (* (`self.DownwardForce`) -1.0)) "None" true)
  (bind (_outhit _returnvalue_2) (`KismetSystemLibrary.LineTraceSingle` :`Start` _returnvalue :`End` (- _returnvalue (0.0 0.0 2000.0)) :`TraceChannel` "TraceTypeQuery1" :`DrawDebugType` "Persistent"))
  (if _returnvalue_2
    (`PrimitiveComponent.AddImpulse` (`self.Ball`) (`KismetMathLibrary.MakeVector` 0.0 0.0 (* (`self.StickyNess`) -1.0)) "None" true)))

(fn `UserConstructionScript`)