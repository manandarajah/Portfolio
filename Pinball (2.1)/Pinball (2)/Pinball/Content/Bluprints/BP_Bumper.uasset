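; BP_Bumper is a pinball bumper that knocks the ball away and awards points when hit.
; A hit from BP_Ball triggers Bump, which applies a velocity-change impulse away from the bumper's center, plays an attached sound and adds score through PinballGameMode.
; A Hit timeline then animates the mechanism's vertical offset, emissive boost and point light intensity together, using a dynamic material created in the construction script.
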(event `self.ReceiveHit`
  (params (MyComp :type "PrimitiveComponent Object Reference") (Other :type "Actor Object Reference") (OtherComp :type "PrimitiveComponent Object Reference") (bSelfMoved :type Boolean) (HitLocation :type "Vector Structure") (HitNormal :type "Vector Structure") (NormalImpulse :type "Vector Structure") (Hit :type "HitResult Structure (by ref)"))
  (bind _asbp_ball (cast `/Game/Bluprints/BP_Ball` Other))
  (`self.Bump` _asbp_ball)
  (bind (_direction _offset) (`Timeline|Hit` :!via `PlayFromStart`)
    (:`Update`
      (`SceneComponent.K2_SetRelativeLocation` (`self.BumperMechanism`) (`KismetMathLibrary.MakeVector` 0.0 0.0 (* _offset -100.0)) false false)
      (`MeshComponent.SetScalarParameterValueOnMaterials` (`self.BumperBase`) "EmissiveBoost" (* _offset 50.0))
      (`LightComponent.SetIntensity` (`self.PointLight`) (* _offset 10000.0)))))

(event `Bump`
  (params (Ball :type "/Game/Bluprints/BP_Ball Object Reference"))
  (`PrimitiveComponent.AddImpulse` (`/Game/Bluprints/BP_Ball.Ball` Ball) (* (`KismetMathLibrary.GetDirectionUnitVector` (`self.K2_GetActorLocation`) (`self.K2_GetActorLocation` Ball)) 2500.0) "None" true)
  (`GameplayStatics.SpawnSoundAttached` "/Game/Assets/BumperCue.BumperCue" (`self.BumperBase`) "None" (0.0 0.0 0.0) (struct) "KeepRelativeOffset" false 1.0 1.0 0.0 null null)
  (bind _aspinball_game_mode (cast `/Game/Bluprints/PinballGameMode` (`GameplayStatics.GetGameMode`)))
  (`/Game/Bluprints/PinballGameMode.AddScore` _aspinball_game_mode 10.0))

(fn `UserConstructionScript`
  (`PrimitiveComponent.CreateDynamicMaterialInstance` (`self.BumperBase`) 0 "/Game/Assets/M_BumperTop.M_BumperTop" "None"))